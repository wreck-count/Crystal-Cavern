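; Collectible crystal that gets pulled into the player and vanishes when the player overlaps it.
; On overlap it caches its location, scale and light intensity, then plays the CrystalCollection timeline.
; The timeline lerps it toward the player pawn's live position while shrinking it to zero, with a separate track fading the light.
; The actor destroys itself when the timeline finishes.
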(event Collision|EventActorBeginOverlap
  (params (OtherActor :type Actor%20Object%20Reference))
  (Utilities|PlayerCheck OtherActor
    (:IsPlayer
      (CallFunction|StoreStartValues)
      (bind (_direction _crystal_progress _light_progress) (Timeline|Crystal%20Collection Play)
        (:Update
          (CallFunction|MoveCrystal _crystal_progress)
          (CallFunction|ScaleCrystal _crystal_progress)
          (CallFunction|ChangeIntensity _light_progress))
        (:Finished
          (Actor|DestroyActor))))))

(fn ConstructionScript)

(fn MoveCrystal
  (params (Alpha :type Float%20%28single-precision%29))
  (Transformation|SetActorLocation (Math|Vector|Lerp(Vector) (Variables|Default|GetStartLocation) (Transformation|GetActorLocation (Game|Player|GetPlayerPawn 0)) Alpha) false false))

(fn StoreStartValues
  (Variables|Default|SetStartLocation (Transformation|GetActorLocation))
  (Variables|Default|SetStartScale (Transformation|GetActorScale3D))
  (Variables|Default|SetStartIntensity (Variables|/Script/Engine.LightComponentBase|GetIntensity (Variables|Default|GetCrystalLight))))

(fn ScaleCrystal
  (params (Alpha :type Float%20%28single-precision%29))
  (Transformation|SetActorScale3D (Math|Vector|Lerp(Vector) (Variables|Default|GetStartScale) "0, 0, 0" Alpha)))

(fn ChangeIntensity
  (params (Alpha :type Float%20%28single-precision%29))
  (Rendering|Components|Light|SetIntensity (Variables|Default|GetCrystalLight) (Math|Float|Lerp (Variables|Default|GetStartIntensity) 0.0 Alpha)))