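; BP_Ball is the player's rolling ball, driven by forward/backward and sideways input.
; Each movement axis, scaled by AccelerationMultiplier, applies torque to the Ball component as an acceleration change, so mass does not affect the response.
; BeginPlay fades the camera in, and any damage to the ball restarts the level through RestartLevel.
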(event Game|Damage|EventAnyDamage
  (params (Damage :type Float%20%28single-precision%29) (DamageType :type Damage%20Type%20Object%20Reference) (InstigatedBy :type Controller%20Object%20Reference) (DamageCauser :type Actor%20Object%20Reference))
  (Utilities|RestartLevel))

(event EventBeginPlay
  (CameraFades|StartCameraFade :self (Game|GetPlayerCameraManager 0) :FromAlpha 1.0 :Duration 1.0))

(event Input|AxisEvents|InputAxisMovementForwards/Backwards
  (params (AxisValue :type Float%20%28single-precision%29))
  (Class|PrimitiveComponent|AddTorqueinRadians (Variables|Default|GetBall) (Math|Vector|MakeVector 0.0 (* AxisValue (Variables|Default|GetAcceleration%20Multiplier)) 0.0) "None" true))

(event Input|AxisEvents|InputAxisMovementSideways
  (params (AxisValue :type Float%20%28single-precision%29))
  (Class|PrimitiveComponent|AddTorqueinRadians (Variables|Default|GetBall) (Math|Vector|MakeVector (* AxisValue (Variables|Default|GetAcceleration%20Multiplier)) 0.0 0.0) "None" true))

(fn ConstructionScript)