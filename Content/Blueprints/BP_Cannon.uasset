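; BP_Cannon is a cannon actor that fires automatically and repeatedly from BeginPlay.
; After each fire-rate delay it spawns an actor at the projectile spawn point, scaled by projectile size, with an explosion effect and sound.
; A recoil timeline then slides the muzzle along its relative Y axis, and its Cannon Fired event track restarts the delay, forming the firing loop.
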(event EventBeginPlay
  (bind _projectilespawnpoint (Variables|Default|GetProjectileSpawnPoint))
  (bind _projectilespawnpoint_2 (Variables|Default|GetProjectileSpawnPoint))
  (bind _returnvalue (Transformation|GetWorldLocation _projectilespawnpoint_2))
  (Utilities|FlowControl|Delay (Variables|CannonProperties|GetProjectileFireRate) :!label _label)
  (Game|SpawnActorfromClass "/Game/Blueprints/Projectiles/BP_CannonProjectile.BP_CannonProjectile_C" (Math|Transform|MakeTransform (Transformation|GetWorldLocation _projectilespawnpoint) (Transformation|GetWorldRotation _projectilespawnpoint) (Math|Conversions|ToVector(Float) (Variables|CannonProperties|GetProjectileSize))) "Undefined" 0 0)
  (Effects|SpawnEmitteratLocation "/Game/StarterContent/Particles/P_Explosion.P_Explosion" _returnvalue (Transformation|GetWorldRotation _projectilespawnpoint_2))
  (Audio|PlaySoundatLocation "/Game/StarterContent/Audio/Explosion_Cue.Explosion_Cue" _returnvalue "0, 0, 0" 1.0 1.0 0.0 0 0 0)
  (bind _recoil_pattern (Timeline|Cannon%20Recoil PlayFromStart)
    (:Update
      (Transformation|SetRelativeLocation (Variables|Default|GetCannonMuzzle) (Math|Vector|MakeVector 0.0 _recoil_pattern 0.0) false false))
    (:Cannon%20Fired
      (goto _label))))

(fn ConstructionScript)